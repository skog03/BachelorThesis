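; Transformer actor for a circuit-building simulation, with four wire terminals and coil meshes that swap by turn count.
; Terminal overlaps record BP_WireUpdated connections and update completion flags, then recheck the circuit.
; A complete circuit is correct when A-side wires link to BP_PowerSupply and B-side wires to BP_Resistor.
; The result goes to the step-down widget if visible, otherwise step-up, which recalculates outputs.
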(event `self.ReceiveBeginPlay`
  (bind _returnvalue (`GameplayStatics.GetActorOfClass` "/Game/Objects/PowerSource/BP_PowerSupply.BP_PowerSupply_C"))
  (set `self.BPPowerSupplyRef` _returnvalue)
  (bind _returnvalue_2 (`GameplayStatics.GetActorOfClass` "/Game/Objects/Resistor/BP_Resistor.BP_Resistor_C"))
  (set `self.BPResistorRef` _returnvalue_2))

(event `self.terminalB2.OnComponentBeginOverlap`
  (params (OverlappedComponent :type "PrimitiveComponent Object Reference") (OtherActor :type "Actor Object Reference") (OtherComp :type "PrimitiveComponent Object Reference") (OtherBodyIndex :type Integer) (bFromSweep :type Boolean) (SweepResult :type "HitResult Structure (by ref)"))
  (`self.startOverlap` OverlappedComponent OtherActor OtherComp)
  (`self.checkCircuitCorrectness` :!label _label))

(event `self.terminalA1.OnComponentBeginOverlap`
  (params (OverlappedComponent :type "PrimitiveComponent Object Reference") (OtherActor :type "Actor Object Reference") (OtherComp :type "PrimitiveComponent Object Reference") (OtherBodyIndex :type Integer) (bFromSweep :type Boolean) (SweepResult :type "HitResult Structure (by ref)"))
  (`self.startOverlap` OverlappedComponent OtherActor OtherComp)
  (`/Game/Objects/BPI_CircuitComponents.checkCircuitCorrectness` :!label _label_2))

(event `self.terminalB2.OnComponentEndOverlap`
  (params (OverlappedComponent :type "PrimitiveComponent Object Reference") (OtherActor :type "Actor Object Reference") (OtherComp :type "PrimitiveComponent Object Reference") (OtherBodyIndex :type Integer))
  (`self.stopOverlap` OverlappedComponent)
  (goto _label))

(event `self.terminalA1.OnComponentEndOverlap`
  (params (OverlappedComponent :type "PrimitiveComponent Object Reference") (OtherActor :type "Actor Object Reference") (OtherComp :type "PrimitiveComponent Object Reference") (OtherBodyIndex :type Integer))
  (`self.stopOverlap` OverlappedComponent)
  (goto _label_2))

(event `self.terminalB1.OnComponentBeginOverlap`
  (params (OverlappedComponent :type "PrimitiveComponent Object Reference") (OtherActor :type "Actor Object Reference") (OtherComp :type "PrimitiveComponent Object Reference") (OtherBodyIndex :type Integer) (bFromSweep :type Boolean) (SweepResult :type "HitResult Structure (by ref)"))
  (`self.startOverlap` OverlappedComponent OtherActor OtherComp)
  (`/Game/Objects/BPI_CircuitComponents.checkCircuitCorrectness` :!label _label_3))

(event `self.terminalA2.OnComponentBeginOverlap`
  (params (OverlappedComponent :type "PrimitiveComponent Object Reference") (OtherActor :type "Actor Object Reference") (OtherComp :type "PrimitiveComponent Object Reference") (OtherBodyIndex :type Integer) (bFromSweep :type Boolean) (SweepResult :type "HitResult Structure (by ref)"))
  (`self.startOverlap` OverlappedComponent OtherActor OtherComp)
  (`/Game/Objects/BPI_CircuitComponents.checkCircuitCorrectness` :!label _label_4))

(event `self.terminalB1.OnComponentEndOverlap`
  (params (OverlappedComponent :type "PrimitiveComponent Object Reference") (OtherActor :type "Actor Object Reference") (OtherComp :type "PrimitiveComponent Object Reference") (OtherBodyIndex :type Integer))
  (`/Game/Objects/BPI_CircuitComponents.stopOverlap` OverlappedComponent)
  (goto _label_3))

(event `self.terminalA2.OnComponentEndOverlap`
  (params (OverlappedComponent :type "PrimitiveComponent Object Reference") (OtherActor :type "Actor Object Reference") (OtherComp :type "PrimitiveComponent Object Reference") (OtherBodyIndex :type Integer))
  (`self.stopOverlap` OverlappedComponent)
  (goto _label_4))

(event `/Game/Objects/BPI_CircuitComponents.checkCircuitCorrectness`
  (bind _wbpstepupref (`self.WBPStepUpRef`))
  (bind _wbpstepupref_2 (`self.WBPStepUpRef`))
  (bind _wbpstepdownref (`self.WBPStepDownRef`))
  (bind _wbpstepdownref_2 (`self.WBPStepDownRef`))
  (if (`self.isCircuitComplete?`)
    (bind _moveon_ (`self.checkCircuitLoop` (`self.A1Wire`) (`self.BPPowerSupplyRef`)))
    (if _moveon_
      (bind _moveon__2 (`self.checkCircuitLoop` (`self.A2Wire`) (`self.BPPowerSupplyRef`)))
      (if _moveon__2
        (bind _moveon__3 (`self.checkCircuitLoop` (`self.B1Wire`) (`self.BPResistorRef`)))
        (if _moveon__3
          (bind _moveon__4 (`self.checkCircuitLoop` (`self.B2Wire`) (`self.BPResistorRef`)))
          (if _moveon__4
            (if (`Widget.IsVisible` _wbpstepdownref)
              (set `/Game/UI/WBP_PlayerUI_StepDown.isCircuitCorrect?` true _wbpstepdownref)
              ; makes sure outputs are shown if user sets sliders before connecting circuit
              (`/Game/UI/WBP_PlayerUI_StepDown.calculateOutputs` _wbpstepdownref)
              (else
                (set `/Game/UI/WBP_PlayerUI_StepUp.isCircuitCorrect?` true _wbpstepupref_2)
                (`/Game/UI/WBP_PlayerUI_StepUp.calculateOutputs` _wbpstepupref_2)))))))
    (elif (`Widget.IsVisible` _wbpstepdownref_2)
      (set `/Game/UI/WBP_PlayerUI_StepDown.isCircuitCorrect?` false _wbpstepdownref_2)
      (`/Game/UI/WBP_PlayerUI_StepDown.calculateOutputs` _wbpstepdownref_2)
      (else
        (set `/Game/UI/WBP_PlayerUI_StepUp.isCircuitCorrect?` false _wbpstepupref)
        (`/Game/UI/WBP_PlayerUI_StepUp.calculateOutputs` _wbpstepupref)))))

(fn `changeLeftMesh`
  (params (Turns :type Integer))
  (if (< Turns 100)
    (`SceneComponent.SetVisibility` (`self.leftTurnsOne`) true false)
    (`SceneComponent.SetVisibility` (`self.leftTurnsTen`) false false)
    (`SceneComponent.SetVisibility` (`self.leftTurnsHundred`) false false)
    (elif (< Turns 2000)
      (`SceneComponent.SetVisibility` (`self.leftTurnsTen`) true false)
      (`SceneComponent.SetVisibility` (`self.leftTurnsOne`) false false)
      (`SceneComponent.SetVisibility` (`self.leftTurnsHundred`) false false)
      (else
        (`SceneComponent.SetVisibility` (`self.leftTurnsHundred`) true false)
        (`SceneComponent.SetVisibility` (`self.leftTurnsOne`) false false)
        (`SceneComponent.SetVisibility` (`self.leftTurnsTen`) false false)))))

(fn `changeRightMesh`
  (params (turns :type Integer))
  (if (< turns 100)
    (`SceneComponent.SetVisibility` (`self.rightTurnsOne`) true false)
    (`SceneComponent.SetVisibility` (`self.rightTurnsTen`) false false)
    (`SceneComponent.SetVisibility` (`self.rightTurnsHundred`) false false)
    (elif (< turns 2000)
      (`SceneComponent.SetVisibility` (`self.rightTurnsTen`) true false)
      (`SceneComponent.SetVisibility` (`self.rightTurnsOne`) false false)
      (`SceneComponent.SetVisibility` (`self.rightTurnsHundred`) false false)
      (else
        (`SceneComponent.SetVisibility` (`self.rightTurnsHundred`) true false)
        (`SceneComponent.SetVisibility` (`self.rightTurnsOne`) false false)
        (`SceneComponent.SetVisibility` (`self.rightTurnsTen`) false false)))))

(fn `checkCircuitLoop`
  (params (wireConnectedAtTerminal :type "/Game/Objects/Wire/BP_WireUpdated Object Reference") (CorrespondingActor :type "Actor Object Reference"))
  (returns (`moveOn?` :type Boolean))
  (bind _endaconnection (`/Game/Objects/Wire/BP_WireUpdated.endAConnection` wireConnectedAtTerminal))
  (if (== _endaconnection self)
    (if (== (`/Game/Objects/Wire/BP_WireUpdated.endBConnection` wireConnectedAtTerminal) CorrespondingActor)
      (return true))
    (elif (== _endaconnection CorrespondingActor)
      (return true))))

(fn `checkIsCompleted`
  (returns (`isCompleted?` :type Boolean))
  (bind _output_get (set `self.isCircuitComplete?` (and (`self.isTransformerComplete?`) (`self.isResistorComplete?`) (`self.isPowerSourceComplete?`))))
  (return _output_get))

(fn `getTerminals`
  (returns (terminals :type "Array of SphereComponent Object Reference"))
  (return (`|MakeArray` (`self.terminalA1`) (`self.terminalA2`) (`self.terminalB1`) (`self.terminalB2`))))

(fn `startOverlap`
  (params (OverlappedComponent :type "PrimitiveComponent Object Reference") (otherActor :type "Actor Object Reference") (otherComponent :type "PrimitiveComponent Object Reference"))
  (returns (`done?` :type Boolean))
  (bind _currentwire (`self.currentWire`))
  (bind _asbp_wire_updated (cast `/Game/Objects/Wire/BP_WireUpdated` otherActor))
  (set `self.currentWire` _asbp_wire_updated)
  (if (== (`/Game/Objects/Wire/BP_WireUpdated.endA` _asbp_wire_updated) otherComponent)
    (set `/Game/Objects/Wire/BP_WireUpdated.endAConnection` self _asbp_wire_updated)
    (else
      (set `/Game/Objects/Wire/BP_WireUpdated.endBConnection` self _asbp_wire_updated)))
  (switch `string` (`KismetSystemLibrary.GetObjectName` OverlappedComponent)
    (:`terminalA1`
      (set `self.A1Wire` _currentwire)
      (set `self.isA1Connected?` true))
    (:`terminalA2`
      (set `self.A2Wire` _currentwire)
      (set `self.isA2Connected?` true))
    (:`terminalB1`
      (set `self.B1Wire` _currentwire)
      (set `self.isB1Connected?` true))
    (:`terminalB2`
      (set `self.B2Wire` _currentwire)
      (set `self.isB2Connected?` true)))
  (if (and (`self.isA1Connected?`) (`self.isA2Connected?`) (`self.isB1Connected?`) (`self.isB2Connected?`))
    (set `self.isTransformerComplete?` true)
    (`self.checkIsCompleted`)
    (return true)))

(fn `stopOverlap`
  (params (overlappedComponent :type "PrimitiveComponent Object Reference"))
  (returns (`done?` :type Boolean))
  (switch `string` (`KismetSystemLibrary.GetObjectName` overlappedComponent)
    (:`terminalA1`
      (set `self.A1Wire` null)
      (set `self.isA1Connected?` false))
    (:`terminalA2`
      (set `self.A2Wire` null)
      (set `self.isA2Connected?` false))
    (:`terminalB1`
      (set `self.B1Wire` null)
      (set `self.isB1Connected?` false))
    (:`terminalB2`
      (set `self.B2Wire` null)
      (set `self.isB2Connected?` false)))
  (set `self.isTransformerComplete?` false)
  (`self.checkIsCompleted`)
  (return true))

(fn `UserConstructionScript`)