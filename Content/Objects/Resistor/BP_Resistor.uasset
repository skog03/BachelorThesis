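; BP_Resistor is a resistor component with Top and Bottom terminals in a wire-connection circuit.
; Terminal overlaps with BP_WireUpdated actors record the wire and register the resistor on the touching wire end.
; With both terminals connected it flags itself complete on the level's BP_Transformer, and ending an overlap clears that flag.
; Each change recomputes overall circuit completion from the transformer's power source, transformer and resistor flags.
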(event `self.ReceiveBeginPlay`
  (bind _returnvalue (`GameplayStatics.GetActorOfClass` "/Game/Objects/Transformer/BP_Transformer.BP_Transformer_C"))
  (set `self.BPTransformerRef` _returnvalue))

(event `self.top.OnComponentBeginOverlap`
  (params (OverlappedComponent :type "PrimitiveComponent Object Reference") (OtherActor :type "Actor Object Reference") (OtherComp :type "PrimitiveComponent Object Reference") (OtherBodyIndex :type Integer) (bFromSweep :type Boolean) (SweepResult :type "HitResult Structure (by ref)"))
  (`self.startOverlap` OverlappedComponent OtherActor OtherComp)
  (`/Game/Objects/BPI_CircuitComponents.NewFunction` (`self.BPTransformerRef`)))

(event `self.top.OnComponentEndOverlap`
  (params (OverlappedComponent :type "PrimitiveComponent Object Reference") (OtherActor :type "Actor Object Reference") (OtherComp :type "PrimitiveComponent Object Reference") (OtherBodyIndex :type Integer))
  (`self.stopOverlap` OverlappedComponent))

(event `self.bottom.OnComponentBeginOverlap`
  (params (OverlappedComponent :type "PrimitiveComponent Object Reference") (OtherActor :type "Actor Object Reference") (OtherComp :type "PrimitiveComponent Object Reference") (OtherBodyIndex :type Integer) (bFromSweep :type Boolean) (SweepResult :type "HitResult Structure (by ref)"))
  (`self.startOverlap` OverlappedComponent OtherActor OtherComp)
  (`/Game/Objects/BPI_CircuitComponents.NewFunction` (`self.BPTransformerRef`)))

(event `self.bottom.OnComponentEndOverlap`
  (params (OverlappedComponent :type "PrimitiveComponent Object Reference") (OtherActor :type "Actor Object Reference") (OtherComp :type "PrimitiveComponent Object Reference") (OtherBodyIndex :type Integer))
  (`self.stopOverlap` OverlappedComponent))

(fn `areAllTerminalsConnected`
  (returns (isConnected :type Boolean))
  (return false))

(fn `fireLoopCheck`
  (returns (NewParam :type Boolean))
  (return false))

(fn `funcCircuitCompletion`
  (returns (`isCompleted?` :type Boolean))
  (bind _bptransformerref (`self.BPTransformerRef`))
  (bind _output_get (set `/Game/Objects/Transformer/BP_Transformer.isCircuitComplete?` (and (`/Game/Objects/Transformer/BP_Transformer.isPowerSourceComplete?` _bptransformerref) (`/Game/Objects/Transformer/BP_Transformer.isTransformerComplete?` _bptransformerref) (`/Game/Objects/Transformer/BP_Transformer.isResistorComplete?` _bptransformerref)) _bptransformerref))
  (return _output_get))

(fn `getTerminals`
  (returns (terminals :type "Array of SphereComponent Object Reference"))
  (return (`|MakeArray` (`self.top`) (`self.bottom`))))

(fn `startOverlap`
  (params (OverlappedComponent :type "PrimitiveComponent Object Reference") (otherActor :type "Actor Object Reference") (otherComponent :type "PrimitiveComponent Object Reference"))
  (returns (`done?` :type Boolean))
  (bind _currentwire (`self.currentWire`))
  (bind _asbp_wire_updated (cast `/Game/Objects/Wire/BP_WireUpdated` otherActor))
  (set `self.currentWire` _asbp_wire_updated)
  (if (== (`/Game/Objects/Wire/BP_WireUpdated.endA` _asbp_wire_updated) otherComponent)
    (set `/Game/Objects/Wire/BP_WireUpdated.endAConnection` self _asbp_wire_updated)
    (else
      (set `/Game/Objects/Wire/BP_WireUpdated.endBConnection` self _asbp_wire_updated)))
  (switch `string` (`KismetSystemLibrary.GetObjectName` OverlappedComponent)
    (:`top`
      (set `self.wireTop` _currentwire)
      (set `self.isTopConnected?` true))
    (:`bottom`
      (set `self.wireBottom` _currentwire)
      (set `self.isBottomConnected?` true)))
  (if (and (`self.isTopConnected?`) (`self.isBottomConnected?`))
    (set `/Game/Objects/Transformer/BP_Transformer.isResistorComplete?` true (`self.BPTransformerRef`))
    (`/Game/Objects/BPI_CircuitComponents.funcCircuitCompletion`)
    (return true)))

(fn `stopOverlap`
  (params (overlappedComponent :type "PrimitiveComponent Object Reference"))
  (returns (`done?` :type Boolean))
  (switch `string` (`KismetSystemLibrary.GetObjectName` overlappedComponent)
    (:`top`
      (set `self.wireTop` null)
      (set `self.isTopConnected?` false))
    (:`bottom`
      (set `self.wireBottom` null)
      (set `self.isBottomConnected?` false)))
  (set `/Game/Objects/Transformer/BP_Transformer.isResistorComplete?` false (`self.BPTransformerRef`))
  (`self.funcCircuitCompletion`)
  (return false))

(fn `UserConstructionScript`)